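; BP_DoorInput is an interactive door that the player swings open and closed with the E key.
; TriggerBox overlaps with BP_ThirdPersonCharacter enable and disable the actor's input, so E only works inside the box.
; A FlipFlop alternately plays and reverses the DoorOpen timeline, which lerps the Door's relative yaw between zero and AngleDoorOpen.
; Opening also prints a "Hello" debug string.
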(event OnComponentBeginOverlap(TriggerBox)
  (params (OverlappedComponent :type Primitive%20Component%20Object%20Reference) (OtherActor :type Actor%20Object%20Reference) (OtherComp :type Primitive%20Component%20Object%20Reference) (OtherBodyIndex :type Integer) (bFromSweep :type Boolean) (SweepResult :type Hit%20Result%20Structure%20%28by%20ref%29))
  (Utilities|Casting|CastToBP_ThirdPersonCharacter OtherActor)
  (Input|EnableInput (Game|GetPlayerController 0)))

(event OnComponentEndOverlap(TriggerBox)
  (params (OverlappedComponent :type Primitive%20Component%20Object%20Reference) (OtherActor :type Actor%20Object%20Reference) (OtherComp :type Primitive%20Component%20Object%20Reference) (OtherBodyIndex :type Integer))
  (Utilities|Casting|CastToBP_ThirdPersonCharacter OtherActor)
  (Input|DisableInput (Game|GetPlayerController 0)))

(event EventBeginPlay)

(event Collision|EventActorBeginOverlap
  (params (OtherActor :type Actor%20Object%20Reference)))

(event EventTick
  (params (DeltaSeconds :type Float%20%28single-precision%29)))

(event Input|KeyboardEvents|E
  (params (Key :type Key%20Structure :default "None"))
  (:Pressed
    (Utilities|FlowControl|FlipFlop
      (:A
        (Development|PrintString "Hello" true true "(R=0.000000,G=0.154264,B=1.000000,A=1.000000)" 3.0)
        (bind _alpha (Timeline|DoorOpen Play)
          (:Update
            (Transformation|SetRelativeRotation (Variables|Default|GetDoor) (Math|Rotator|MakeRotator 0.0 0.0 (Math|Float|Lerp 0.0 (Variables|Default|GetAngleDoorOpen) _alpha)) false false))))
      (:B
        (Timeline|DoorOpen Reverse)))))

(fn ConstructionScript)