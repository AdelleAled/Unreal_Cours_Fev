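; Door actor that swings open when anything begins overlapping its TriggerBox, also printing a debug "Hello".
; The DoorOpen timeline lerps the Door's relative yaw from zero to AngleDoorOpen.
; Five seconds after the timeline finishes, one SetRelativeRotation call resets the yaw without animation, using a hardcoded lerp start instead of AngleDoorOpen.
; Leftover disconnected timeline, delay and rotation nodes never run.
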(event OnComponentBeginOverlap(TriggerBox)
  (params (OverlappedComponent :type Primitive%20Component%20Object%20Reference) (OtherActor :type Actor%20Object%20Reference) (OtherComp :type Primitive%20Component%20Object%20Reference) (OtherBodyIndex :type Integer) (bFromSweep :type Boolean) (SweepResult :type Hit%20Result%20Structure%20%28by%20ref%29))
  (bind _door (Variables|Default|GetDoor))
  (Development|PrintString "Hello" true true "(R=0.000000,G=0.154264,B=1.000000,A=1.000000)" 3.0)
  (bind _alpha (Timeline|DoorOpen Play)
    (:Update
      (Transformation|SetRelativeRotation _door (Math|Rotator|MakeRotator 0.0 0.0 (Math|Float|Lerp 0.0 (Variables|Default|GetAngleDoorOpen) _alpha)) false false))
    (:Finished
      (Utilities|FlowControl|Delay 5.0)
      (Transformation|SetRelativeRotation _door (Math|Rotator|MakeRotator 0.0 0.0 (Math|Float|Lerp 1e+02 0.0 _alpha)) false false))))

(event EventBeginPlay)

(event Collision|EventActorBeginOverlap
  (params (OtherActor :type Actor%20Object%20Reference)))

(event EventTick
  (params (DeltaSeconds :type Float%20%28single-precision%29)))

(fn ConstructionScript)